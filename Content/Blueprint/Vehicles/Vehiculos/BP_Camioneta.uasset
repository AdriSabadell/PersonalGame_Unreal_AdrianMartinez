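; BP_Camioneta is a vehicle actor that moves along the spline of a referenced actor.
; BeginPlay runs a GetActorOfClass lookup, sets SplineREF to None rather than to that result, then calls MoveObject.
; MoveObject plays a timeline at a rate of 1/TimeToComplete, mapping its track onto spline length to set the transform each update.
; Location is sampled in world space, while rotation is sampled in local space.
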(event Custom|MoveObject
  (bind _splineref (Variables|Default|GetSplineREF))
  (bind _spline (Variables|Components|GetSpline _splineref))
  (Components|Timeline|SetPlayRate (Variables|Default|GetMoveObjetctT) (/ 1.0 (Variables|Default|GetTimeToComplete)))
  (bind _movetrack (Timeline|MoveObjetctT Play)
    (:Update
      (Transformation|SetActorTransform (Math|Transform|MakeTransform (Spline|GetLocationatDistanceAlongSpline _spline (Math|Float|Lerp 0.0 (Spline|GetSplineLength (Variables|Components|GetSpline (.SplineREF (Variables|Default|GetSplineREF)))) _movetrack) "World") (Spline|GetRotationatDistanceAlongSpline _spline (Math|Float|Lerp 0.0 (Spline|GetSplineLength (Variables|Components|GetSpline (.SplineREF (Variables|Default|GetSplineREF)))) _movetrack) "Local") "1.000000,1.000000,1.000000")))))

(event EventBeginPlay
  (bind _returnvalue (Actor|GetActorOfClass 0))
  (Variables|Default|SetSplineREF 0 _returnvalue)
  (CallFunction|MoveObject))

(fn ConstructionScript)